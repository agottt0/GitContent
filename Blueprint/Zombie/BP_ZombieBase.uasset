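; BP_ZombieBase is a zombie base Blueprint that handles health, damage, death and hit reactions.
; AnyDamage subtracts damage from current health, clamps it to the maximum in the zombie's FGetZombieInfo entry, prints debug output and calls Death at zero.
; Death destroys the actor, or resets health from an empty-name info lookup when passed false.
; A separate event plays a hit-react montage for Head bone hits.
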(event `SetZombieHealth`
  (params (CurrentZombieHealth :type "Float (double-precision)"))
  (set `self.CurrentZombieHealth` CurrentZombieHealth))

(event `self.ReceiveAnyDamage`
  (params (Damage :type "Float (single-precision)") (DamageType :type "DamageType Object Reference") (InstigatedBy :type "Controller Object Reference") (DamageCauser :type "Actor Object Reference"))
  (bind _currentzombiehealth (`self.CurrentZombieHealth`))
  (`KismetSystemLibrary.PrintString` "Apply")
  (`self.SetZombieHealth` (`KismetMathLibrary.FClamp` (- (`self.CurrentZombieHealth`) Damage) 0.0 (`.MaximumHealth_15_C6F1CD93467C3BE5F66B4FBC44253295` (break `/Game/GitContent/Data/ST_Zombie` (`/Game/GitContent/Blueprint/Library/BP_FunctionLibrary.f_GetZombieInfo` (`self.ZombieName`))))))
  (`KismetSystemLibrary.PrintString` (`KismetStringLibrary.Conv_DoubleToString` _currentzombiehealth))
  (if (<= _currentzombiehealth 0.0)
    (`self.Death` true)))

(event `Death`
  (params (bIsDead :type Boolean))
  (bind _output_get (set `self.bIsDead` bIsDead))
  (if _output_get
    (`self.K2_DestroyActor`)
    (else
      (`self.SetZombieHealth` (`.MaximumHealth_15_C6F1CD93467C3BE5F66B4FBC44253295` (break `/Game/GitContent/Data/ST_Zombie` (`/Game/GitContent/Blueprint/Library/BP_FunctionLibrary.f_GetZombieInfo` "")))))))

(event `PlayZombieHitReactAnim`
  (params (BoneName :type Name))
  (switch `name` BoneName
    (:`Head`
      (`|PlayMontage` (`self.Mesh`) "/Game/GitContent/Animations/EnemyAnim/Animations/Action/AnimMon_Zombie_HitReact_Head.AnimMon_Zombie_HitReact_Head"))))

(fn `UserConstructionScript`)