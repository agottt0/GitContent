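; PC_SurviveGame is the player controller for a survival game, owning the player HUD and pause widgets.
; It shows the HUD on BeginPlay, and a show/hide event lazily creates, caches and adds each widget to the viewport or removes it by enum.
; Other events forward weapon type and thumbnail, crosshair visibility and hit feedback to the player HUD.
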(event `self.ReceiveBeginPlay`
  (`self.ShowHideWidgets` "NewEnumerator0" true))

(event `ShowHideWidgets`
  (params (Widget :type "/Game/GitContent/Data/Enum_UI Enum" :default "NewEnumerator0") (Show :type Boolean))
  (if Show
    (`self.f_ShowWidget` Widget)
    (else
      (`self.f_HideWidget` Widget))))

(event `UpdateWeaponUI`
  (params (CurrentWeapon :type "/Game/GitContent/Blueprint/Weapon/BP_WeaponBase Object Reference"))
  (bind ((`Type_52_DEF4F6DB403B2ABF457F1D91EC2601DD` _type) (`Thumbnail_72_5A8D8AAD4C892067B9FEF69FE01BF449` _thumbnail)) (break `/Game/GitContent/Data/ST_Weapon` (`/Game/GitContent/Blueprint/Library/BP_FunctionLibrary.f_GetWeaponInfo` (`/Game/GitContent/Blueprint/Weapon/BP_WeaponBase.WeaponName` CurrentWeapon))))
  (`/Game/GitContent/UI/WB_Player.UpdateWeaponUI` (`self.WB_Player`) _type _thumbnail))

(event `DisplayCrossHairUI`
  (params (Display :type Boolean))
  (`/Game/GitContent/UI/WB_Player.DisplayCrossHairUI` (`self.WB_Player`) Display))

(event `DisplayHittingUI`
  (`/Game/GitContent/UI/WB_Player.DisplayHittingUI` (`self.WB_Player`)))

(fn `f_GetPlayerControllerRef`
  (returns (PlayerController :type "/Blueprint/PC_SurviveGame Object Reference"))
  (return self))

(fn `f_HideWidget`
  (params (Widget :type "/Game/GitContent/Data/Enum_UI Enum" :default "NewEnumerator0"))
  (switch `/Game/GitContent/Data/Enum_UI` Widget
    (:`NewEnumerator0`
      (bind _wb_player (`self.WB_Player`)
        (:`then`
          (`Widget.RemoveFromParent` _wb_player))
        (:`else`)))
    (:`NewEnumerator1`
      (bind _wb_pause (`self.WB_Pause`)
        (:`then`
          (`Widget.RemoveFromParent` _wb_pause))
        (:`else`)))))

(fn `f_ShowWidget`
  (params (Widget :type "/Game/GitContent/Data/Enum_UI Enum" :default "NewEnumerator0"))
  (switch `/Game/GitContent/Data/Enum_UI` Widget
    (:`NewEnumerator0`
      (`self.WB_Player`
        (:`then`
          _)
        (:`else`
          (bind _returnvalue (`|CreateWidget` "/Game/GitContent/UI/WB_Player.WB_Player_C"))
          (bind _output_get (set `self.WB_Player` _returnvalue))))
      (`UserWidget.AddToViewport` _output_get 0))
    (:`NewEnumerator1`
      (`self.WB_Pause`
        (:`then`
          _)
        (:`else`
          (bind _returnvalue_2 (`|CreateWidget` "/Game/GitContent/UI/WB_Pause.WB_Pause_C"))
          (bind _output_get_2 (set `self.WB_Pause` _returnvalue_2))))
      (`UserWidget.AddToViewport` _output_get_2 0))))

(fn `UserConstructionScript`)