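; Base weapon actor built from modular part meshes such as hull, magazine, barrel, grips and sight.
; Hover and unhover events toggle a highlight by writing custom depth stencil values on the parts; the click event is empty.
; Helper functions switch physics and collision across the parts, excluding Melee, which is only highlighted.
; Scaling applies to the Hull alone, and a getter returns a self reference.
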(event `/Game/GitContent/Blueprint/Interface/INT_RayDetection.Event_Hover`
  (`self.f_SetHighLight` 1))

(event `/Game/GitContent/Blueprint/Interface/INT_RayDetection.Event_Click`)

(event `/Game/GitContent/Blueprint/Interface/INT_RayDetection.Event_Unhover`
  (`self.f_SetHighLight` 0))

(fn `f_GetWeaponBaseRef`
  (returns (WeaponBase :type "/Blueprint/Weapon/BP_WeaponBase Object Reference"))
  (return self))

(fn `f_SetCollison`
  (params (NewType :type "ECollisionEnabled Enum" :default "NoCollision"))
  (`PrimitiveComponent.SetCollisionEnabled` (`self.Cube`) NewType)
  (`PrimitiveComponent.SetCollisionEnabled` (`self.Hull`) NewType)
  (`PrimitiveComponent.SetCollisionEnabled` (`self.MagMount`) NewType)
  (`PrimitiveComponent.SetCollisionEnabled` (`self.Barrel`) NewType)
  (`PrimitiveComponent.SetCollisionEnabled` (`self.BarrelAttach`) NewType)
  (`PrimitiveComponent.SetCollisionEnabled` (`self.Mag`) NewType)
  (`PrimitiveComponent.SetCollisionEnabled` (`self.Butt`) NewType)
  (`PrimitiveComponent.SetCollisionEnabled` (`self.Grip`) NewType)
  (`PrimitiveComponent.SetCollisionEnabled` (`self.HandGuard`) NewType)
  (`PrimitiveComponent.SetCollisionEnabled` (`self.FrontGrip`) NewType)
  (`PrimitiveComponent.SetCollisionEnabled` (`self.Sight`) NewType))

(fn `f_SetHighLight`
  (params (Value :type Integer))
  (bind _hull (`self.Hull`))
  (bind _magmount (`self.MagMount`))
  (bind _mag (`self.Mag`))
  (bind _melee (`self.Melee`))
  (bind _butt (`self.Butt`))
  (bind _grip (`self.Grip`))
  (bind _handguard (`self.HandGuard`))
  (bind _frontgrip (`self.FrontGrip`))
  (bind _barrel (`self.Barrel`))
  (bind _barrelattach (`self.BarrelAttach`))
  (bind _sight (`self.Sight`))
  (`|ExecutionSequence`
    (:`then_0`
      (`PrimitiveComponent.SetRenderCustomDepth` _hull true)
      (`PrimitiveComponent.SetCustomDepthStencilValue` _hull Value))
    (:`then_1`
      (`PrimitiveComponent.SetRenderCustomDepth` _magmount true)
      (`PrimitiveComponent.SetCustomDepthStencilValue` _magmount Value))
    (:`then_2`
      (`PrimitiveComponent.SetCustomDepthStencilValue` _mag Value :!label _label))
    (:`then_3`
      (`PrimitiveComponent.SetRenderCustomDepth` _mag true)
      (goto _label))
    (:`then_4`
      (`PrimitiveComponent.SetRenderCustomDepth` _butt true)
      (`PrimitiveComponent.SetCustomDepthStencilValue` _butt Value))
    (:`then_5`
      (`PrimitiveComponent.SetRenderCustomDepth` _grip true)
      (`PrimitiveComponent.SetCustomDepthStencilValue` _grip Value))
    (:`then_6`
      (`PrimitiveComponent.SetRenderCustomDepth` _handguard true)
      (`PrimitiveComponent.SetCustomDepthStencilValue` _handguard Value))
    (:`then_7`
      (`PrimitiveComponent.SetRenderCustomDepth` _frontgrip true)
      (`PrimitiveComponent.SetCustomDepthStencilValue` _frontgrip Value))
    (:`then_8`
      (`PrimitiveComponent.SetRenderCustomDepth` _barrel true)
      (`PrimitiveComponent.SetCustomDepthStencilValue` _barrel Value))
    (:`then_9`
      (`PrimitiveComponent.SetRenderCustomDepth` _barrelattach true)
      (`PrimitiveComponent.SetCustomDepthStencilValue` _barrelattach Value))
    (:`then_10`
      (`PrimitiveComponent.SetRenderCustomDepth` _sight true)
      (`PrimitiveComponent.SetCustomDepthStencilValue` _sight Value))
    (:`then_11`
      (`PrimitiveComponent.SetRenderCustomDepth` _melee true)
      (`PrimitiveComponent.SetCustomDepthStencilValue` _melee Value))))

(fn `f_SetScale`
  (params (NewScale3D :type "Vector Structure"))
  (`SceneComponent.SetRelativeScale3D` (`self.Hull`) NewScale3D))

(fn `f_SetSimulatePhysics`
  (params (SetPhysics :type Boolean))
  (`PrimitiveComponent.SetSimulatePhysics` (`self.Cube`) SetPhysics)
  (`PrimitiveComponent.SetSimulatePhysics` (`self.Hull`) SetPhysics)
  (`PrimitiveComponent.SetSimulatePhysics` (`self.MagMount`) SetPhysics)
  (`PrimitiveComponent.SetSimulatePhysics` (`self.Mag`) SetPhysics)
  (`PrimitiveComponent.SetSimulatePhysics` (`self.Butt`) SetPhysics)
  (`PrimitiveComponent.SetSimulatePhysics` (`self.Grip`) SetPhysics)
  (`PrimitiveComponent.SetSimulatePhysics` (`self.HandGuard`) SetPhysics)
  (`PrimitiveComponent.SetSimulatePhysics` (`self.FrontGrip`) SetPhysics)
  (`PrimitiveComponent.SetSimulatePhysics` (`self.Barrel`) SetPhysics)
  (`PrimitiveComponent.SetSimulatePhysics` (`self.BarrelAttach`) SetPhysics)
  (`PrimitiveComponent.SetSimulatePhysics` (`self.Sight`) SetPhysics))

(fn `UserConstructionScript`)