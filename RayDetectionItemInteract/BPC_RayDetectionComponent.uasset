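; Scene component that lets the player hover over and click actors in view, using a sphere trace.
; While toggled on, it ticks at a set interval, tracing for chosen object types from its location along player 0's control rotation.
; Changes in the hit actor send hover and unhover messages, evaluated before each new trace so they lag one tick.
; Click events message the current hit, and switching off unhovers it.
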(event `Event_StartTick`
  (params (IsStart :type Boolean))
  (`self.SetComponentTickEnabled` IsStart)
  (if IsStart
    (`self.SetComponentTickInterval` (`self.Tick Interval`))
    (else
      (bind _hit_actor (`self.Hit Actor`)
        (:`then`
          (message `/Game/GitContent/Blueprint/Interface/INT_RayDetection.Event_Unhover` _hit_actor)
          (set `self.Hit Actor` null))
        (:`else`
          _))
      (set `self.Last Hit Actor` null))))

(event `self.ReceiveTick`
  (params (DeltaSeconds :type "Float (single-precision)"))
  (bind (_raystart _rayend) (`self.Fun_RayStartToEnd`))
  (`self.Fun_CheckIfHover`)
  (bind (_outhit _returnvalue) (`KismetSystemLibrary.SphereTraceSingleForObjects` :`Start` _raystart :`End` _rayend :`ObjectTypes` (`self.DetectionObject`) :`bTraceComplex` (`self.Trace Complex`) :`DrawDebugType` (`self.Draw Debug Type`) :`TraceColor` (`self.Trace Color`) :`TraceHitColor` (`self.Trace Hit Color`) :`DrawTime` (`self.Draw Time`)))
  (if _returnvalue
    (set `self.Hit Actor` (`.HitActor` (`GameplayStatics.BreakHitResult` _outhit)))
    (else
      (set `self.Hit Actor` null))))

(event `Event_Click`
  (bind _hit_actor (`self.Hit Actor`)
    (:`then`
      (message `/Game/GitContent/Blueprint/Interface/INT_RayDetection.Event_Click` _hit_actor))
    (:`else`)))

(fn `Fun_CheckIfHover`
  (bind _hit_actor (`self.Hit Actor`))
  (`self.Hit Actor`
    (:`then`
      (bind _last_hit_actor (`self.Last Hit Actor`)
        (:`then`
          (if (not (== (`self.Hit Actor`) _last_hit_actor))
            (message `/Game/GitContent/Blueprint/Interface/INT_RayDetection.Event_Unhover` (`self.Last Hit Actor`))
            (message `/Game/GitContent/Blueprint/Interface/INT_RayDetection.Event_Hover` _hit_actor)
            (set `self.Last Hit Actor` _hit_actor)))
        (:`else`
          (message `/Game/GitContent/Blueprint/Interface/INT_RayDetection.Event_Hover` (`self.Hit Actor`))
          (set `self.Last Hit Actor` (`self.Hit Actor`)))))
    (:`else`
      (bind _last_hit_actor_2 (`self.Last Hit Actor`)
        (:`then`
          (message `/Game/GitContent/Blueprint/Interface/INT_RayDetection.Event_Unhover` _last_hit_actor_2)
          (set `self.Last Hit Actor` null))
        (:`else`)))))

(fn `Fun_RayStartToEnd`
  (returns (RayStart :type "Vector Structure") (RayEnd :type "Vector Structure"))
  (bind _returnvalue (`self.K2_GetComponentLocation`))
  (return _returnvalue (+ _returnvalue (* (`KismetMathLibrary.GetForwardVector` (`Controller.GetControlRotation` (`GameplayStatics.GetPlayerController` 0))) (`self.DetectionDistance`)))))